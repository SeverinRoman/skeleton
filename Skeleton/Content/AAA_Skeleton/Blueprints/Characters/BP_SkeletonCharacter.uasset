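; BP_SkeletonCharacter is a controllable skeleton character built from separate skeletal mesh body parts.
; Enhanced Input actions drive camera yaw and pitch and forward movement input to BPMoveComponent, which also handles switching between sprint and run as the run input starts and completes.
; The construction script sets the main Mesh as leader pose for every bone-piece mesh, so the modular body animates as one.
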(event `EnhancedInput|/Game/AAA_Skeleton/Blueprints/Input/Actions/IA_Move`
  (params (ActionValue :type "Vector2D Structure") (ElapsedSeconds :type "Float (double-precision)") (TriggeredSeconds :type "Float (double-precision)") (InputAction :type "InputAction Object Reference" :default "/Game/AAA_Skeleton/Blueprints/Input/Actions/IA_Move.IA_Move"))
  (:`Triggered`
    (`MoveComponent.Move` (`self.BP_MoveComponent`) ActionValue_X ActionValue_Y)))

(event `EnhancedInput|/Game/AAA_Skeleton/Blueprints/Input/Actions/IA_Camera`
  (params (ActionValue :type "Vector2D Structure") (ElapsedSeconds :type "Float (double-precision)") (TriggeredSeconds :type "Float (double-precision)") (InputAction :type "InputAction Object Reference" :default "/Game/AAA_Skeleton/Blueprints/Input/Actions/IA_Camera.IA_Camera"))
  (:`Triggered`
    (`self.AddControllerYawInput` ActionValue_X)
    (`self.AddControllerPitchInput` ActionValue_Y)))

(event `EnhancedInput|/Game/AAA_Skeleton/Blueprints/Input/Actions/IA_Run`
  (params (ActionValue :type Boolean) (ElapsedSeconds :type "Float (double-precision)") (TriggeredSeconds :type "Float (double-precision)") (InputAction :type "InputAction Object Reference" :default "/Game/AAA_Skeleton/Blueprints/Input/Actions/IA_Run.IA_Run"))
  (bind _bp_movecomponent (`self.BP_MoveComponent`))
  (:`Started`
    (`MoveComponent.Sprint` _bp_movecomponent))
  (:`Completed`
    (`MoveComponent.Run` _bp_movecomponent)))

(fn `UserConstructionScript`
  (`SkinnedMeshComponent.SetLeaderPoseComponent` (`self.SKM_Skeleton_Body_ShinLt`) (`self.Mesh`) false false)
  (`SkinnedMeshComponent.SetLeaderPoseComponent` (`self.SKM_Skeleton_Body_CollarboneRt`) (`self.Mesh`) false false)
  (`SkinnedMeshComponent.SetLeaderPoseComponent` (`self.SKM_Skeleton_Body_ElbowLt`) (`self.Mesh`) false false)
  (`SkinnedMeshComponent.SetLeaderPoseComponent` (`self.SKM_Skeleton_Body_ElbowRt`) (`self.Mesh`) false false)
  (`SkinnedMeshComponent.SetLeaderPoseComponent` (`self.SKM_Skeleton_Body_HipLt`) (`self.Mesh`) false false)
  (`SkinnedMeshComponent.SetLeaderPoseComponent` (`self.SKM_Skeleton_Body_HipLt1`) (`self.Mesh`) false false)
  (`SkinnedMeshComponent.SetLeaderPoseComponent` (`self.SKM_Skeleton_Body_HipRt`) (`self.Mesh`) false false)
  (`SkinnedMeshComponent.SetLeaderPoseComponent` (`self.SKM_Skeleton_Body_HipRt1`) (`self.Mesh`) false false)
  (`SkinnedMeshComponent.SetLeaderPoseComponent` (`self.SKM_Skeleton_Body_Jaw_Hidden`) (`self.Mesh`) false false)
  (`SkinnedMeshComponent.SetLeaderPoseComponent` (`self.SKM_Skeleton_Body_CollarboneLt`) (`self.Mesh`) false false)
  (`SkinnedMeshComponent.SetLeaderPoseComponent` (`self.SKM_Skeleton_Body_ShinRt`) (`self.Mesh`) false false)
  (`SkinnedMeshComponent.SetLeaderPoseComponent` (`self.SKM_Skeleton_Body_ShoulderLt`) (`self.Mesh`) false false)
  (`SkinnedMeshComponent.SetLeaderPoseComponent` (`self.SKM_Skeleton_Body_ShoulderRt`) (`self.Mesh`) false false)
  (`SkinnedMeshComponent.SetLeaderPoseComponent` (`self.SKM_Skeleton_Body_Skull`) (`self.Mesh`) false false)
  (`SkinnedMeshComponent.SetLeaderPoseComponent` (`self.SKM_Skeleton_Body_TibiaLt`) (`self.Mesh`) false false)
  (`SkinnedMeshComponent.SetLeaderPoseComponent` (`self.SKM_Skeleton_Body_TibiaRt`) (`self.Mesh`) false false)
  (`SkinnedMeshComponent.SetLeaderPoseComponent` (`self.SKM_Skeleton_Body_WristsLt`) (`self.Mesh`) false false)
  (`SkinnedMeshComponent.SetLeaderPoseComponent` (`self.SKM_Skeleton_Body_WristsRt`) (`self.Mesh`) false false)
  (`SkinnedMeshComponent.SetLeaderPoseComponent` (`self.SKM_Skeleton_Body_Bone`) (`self.Mesh`) false false))