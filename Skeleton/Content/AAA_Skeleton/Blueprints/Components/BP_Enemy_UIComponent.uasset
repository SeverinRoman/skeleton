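; Enemy UI component that drives a world-space health bar on its owning actor.
; After a short delay on BeginPlay, it finds the owner's health and widget components and caches the WBP_World_Health widget.
; Health change events push the health percentage into the widget.
; Each tick, it billboards the widget component by rotating it toward the player camera.
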(event `self.ReceiveBeginPlay`
  (`KismetSystemLibrary.Delay` 0.1)
  (`self.BP_Init`)
  (add `HealthComponent.OnHealthChange` (`self.HealthComponent`) (delegate `OnHealthChange`))
  (`self.BP_UpdateHealth`))

(event `OnHealthChange`
  (`self.BP_UpdateHealth`))

(event `self.ReceiveTick`
  (params (DeltaSeconds :type "Float (single-precision)"))
  (`self.BP_UpdateRotation`))

(fn `BP_Init`
  (bind _output_get (set `self.Owner` (`self.GetOwner`)))
  (`/Engine/EditorBlueprintResources/StandardMacros.IsValid` _output_get
    (:`Is Valid`
      (set `self.HealthComponent` (`Actor.GetComponentByClass` (`self.Owner`) "/Game/AAA_Skeleton/Blueprints/Components/BP_HealthComponent.BP_HealthComponent_C"))
      (bind _output_get_2 (set `self.WidgetComponent` (`Actor.GetComponentByClass` (`self.Owner`) "/Script/UMG.WidgetComponent")))
      (bind _output_get_3 (set `self.UserWidget` (`WidgetComponent.GetWidget` _output_get_2)))
      (bind _aswbp_world_health (cast `/Game/AAA_Skeleton/Blueprints/UI/WBP_World_Health` _output_get_3))
      (set `self.WBP World Health` _aswbp_world_health))))

(fn `BP_UpdateHealth`
  (`/Engine/EditorBlueprintResources/StandardMacros.IsValid` (`self.HealthComponent`)
    (:`Is Valid`
      (`/Engine/EditorBlueprintResources/StandardMacros.IsValid` (`self.WBP World Health`)
        (:`Is Valid`
          (set `/Game/AAA_Skeleton/Blueprints/UI/WBP_World_Health.Health` (`HealthComponent.GetPercentHealth` (`self.HealthComponent`)) (`self.WBP World Health`)))))))

(fn `BP_UpdateRotation`
  (bind _widgetcomponent (`self.WidgetComponent`))
  (`/Engine/EditorBlueprintResources/StandardMacros.IsValid` (`self.WidgetComponent`)
    (:`Is Valid`
      (`SceneComponent.K2_SetWorldRotation` _widgetcomponent (`KismetMathLibrary.FindLookAtRotation` (`SceneComponent.K2_GetComponentLocation` _widgetcomponent) (`SceneComponent.K2_GetComponentLocation` (`PlayerCameraManager.TransformComponent` (`GameplayStatics.GetPlayerCameraManager` 0)))) false false))))